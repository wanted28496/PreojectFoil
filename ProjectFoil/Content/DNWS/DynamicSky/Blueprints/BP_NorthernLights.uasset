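; Northern lights actor for the dynamic sky that fades in on spawn and fades out before destroying itself.
; The construction script scatters a random number of huge, randomly scaled mesh instances around an anchor point, with offset range growing per index.
; After a short delay, BeginPlay creates a dynamic material, sets its texture and drives opacity to a random target through the Fadein timeline.
; Despawn reverses that timeline and destroys the actor after a delay.
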(event `self.ReceiveBeginPlay`
  (`KismetSystemLibrary.Delay` 0.2)
  (set `self.Opacity value` (`KismetMathLibrary.RandomFloatInRange` 0.6 0.75))
  (bind _returnvalue (`PrimitiveComponent.CreateDynamicMaterialInstance` (`self.NLights`) 0 "/Game/DNWS/DynamicSky/Textures/Materials/M_NorthernLightsMat_Inst.M_NorthernLightsMat_Inst" "None"))
  (bind _output_get (set `self.MatInst` _returnvalue))
  (`MaterialInstanceDynamic.SetTextureParameterValue` _output_get "Texture" (`self.NLightsTex`))
  (bind (_direction _fade) (`Timeline|Fadein` :!via `PlayFromStart` :!label _label)
    (:`Update`
      (`MaterialInstanceDynamic.SetScalarParameterValue` _output_get "Opacity" (`KismetMathLibrary.Lerp` 0.0 (`self.Opacity value`) _fade)))))

(event `Despawn`
  (`|ExecutionSequence`
    (:`then_0`
      (goto _label :!via `ReverseFromEnd`))
    (:`then_1`
      (`KismetSystemLibrary.Delay` 2.0)
      (`self.K2_DestroyActor`))))

(fn `UserConstructionScript`
  (bind _returnvalue (`KismetMathLibrary.RandomFloatInRange` 6500.0 8500.0))
  (bind (_relativelocation_x _relativelocation_y _relativelocation_z) (`KismetMathLibrary.BreakVector` (`SceneComponent.RelativeLocation` (`self.AnchorPoint`))))
  ;[1 1 1] Spawning Northern Lights
  (for _index (range (+ (`KismetMathLibrary.RandomIntegerInRange` 10 16) 1))
    (`InstancedStaticMeshComponent.AddInstance` (`self.NLights`) (`KismetMathLibrary.MakeTransform` (`KismetMathLibrary.MakeVector` (+ _relativelocation_x (`KismetMathLibrary.Conv_IntToDouble` (* (* _index 25) (`KismetMathLibrary.RandomIntegerInRange` -10000 10000)))) (+ _relativelocation_y (`KismetMathLibrary.Conv_IntToDouble` (* (* _index 25) (`KismetMathLibrary.RandomIntegerInRange` -10000 10000)))) _relativelocation_z) (struct) (`KismetMathLibrary.MakeVector` _returnvalue _returnvalue _returnvalue)))))