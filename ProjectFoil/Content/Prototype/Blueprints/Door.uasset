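; Prototype interactable door that player 0 opens with E while input is enabled by a trigger box overlap, with no check on the overlapping actor.
; Pressing E plays the skeletal door animation and lets pawns through the collider.
; After a fixed delay it restores blocking, snaps the pose back by resetting the skeletal mesh and plays the close sound.
; The open sound plays on key release.
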(event `self.Box.OnComponentBeginOverlap`
  (params (OverlappedComponent :type "PrimitiveComponent Object Reference") (OtherActor :type "Actor Object Reference") (OtherComp :type "PrimitiveComponent Object Reference") (OtherBodyIndex :type Integer) (bFromSweep :type Boolean) (SweepResult :type "HitResult Structure (by ref)"))
  (`self.EnableInput` (`GameplayStatics.GetPlayerController` 0)))

(event `Key|E`
  (params (Key :type "Key Structure"))
  (:`Pressed`
    (`SkeletalMeshComponent.PlayAnimation` (`self.Door_Anim_02`) "/Game/Geometry/Shell_Sections/DoorTest_Anim/Door_Anim_02_Anim.Door_Anim_02_Anim" false)
    (`PrimitiveComponent.SetCollisionResponseToChannel` (`self.doorCollider`) "ECC_Pawn" "ECR_Ignore")
    (`KismetSystemLibrary.Delay` 4.0)
    (`PrimitiveComponent.SetCollisionResponseToChannel` (`self.doorCollider`) "ECC_Pawn" "ECR_Block")
    (`SkinnedMeshComponent.SetSkinnedAssetAndUpdate` (`self.Door_Anim_02`) "/Game/Geometry/Shell_Sections/DoorTest_Anim/Door_Anim_02.Door_Anim_02" true)
    (`GameplayStatics.PlaySound2D` "/Game/Prototype/Audio/door_close_v1.door_close_v1" 1.0 1.0 0.0 null null))
  (:`Released`
    (`GameplayStatics.PlaySound2D` "/Game/Prototype/Audio/dooropen.dooropen" 1.0 1.0 0.0 null null)))

(event `self.Box.OnComponentEndOverlap`
  (params (OverlappedComponent :type "PrimitiveComponent Object Reference") (OtherActor :type "Actor Object Reference") (OtherComp :type "PrimitiveComponent Object Reference") (OtherBodyIndex :type Integer))
  (`self.DisableInput` (`GameplayStatics.GetPlayerController` 0)))

(fn `UserConstructionScript`)