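; Warning light actor that spins with an alarm sound and can be blown out.
; When EnableLight is set, BeginPlay starts a looping timer that yaws the Rotator by RotationSpeed and spawns the warning sound.
; Otherwise the point light is hidden in the construction script and destroyed at BeginPlay.
; The Explosion event plays a blast sound, then after a delay spawns spark and smoke effects, destroys the light and stops the alarm.
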(event `self.ReceiveBeginPlay`
  (if (`self.Enable light`)
    (`KismetSystemLibrary.K2_SetTimer` null "Rotate" 0.025 true)
    (bind _returnvalue (`GameplayStatics.SpawnSoundAtLocation` "/Game/Prototype/Audio/Warning_light_Cue.Warning_light_Cue" (`self.K2_GetActorLocation` self) (struct) 1.0 1.0 0.0 null null))
    (set `self.Warning sound` _returnvalue)
    (else
      (`ActorComponent.K2_DestroyComponent` (`self.PointLight`)))))

(event `Explosion`
  (bind _returnvalue (`self.K2_GetActorLocation` self))
  (`GameplayStatics.SpawnSoundAtLocation` "/Game/Prototype/Audio/alarmExplosion_Cue.alarmExplosion_Cue" _returnvalue (struct) 1.0 1.0 0.0 null null)
  (`KismetSystemLibrary.Delay` 1.0)
  (`GameplayStatics.SpawnEmitterAtLocation` "/Game/Prototype/VFX/P_SparkExplosion.P_SparkExplosion" _returnvalue)
  (`GameplayStatics.SpawnEmitterAtLocation` "/Game/Prototype/VFX/P_Smoke.P_Smoke" _returnvalue)
  (`ActorComponent.K2_DestroyComponent` (`self.PointLight`))
  (`AudioComponent.Stop` (`self.Warning sound`)))

(fn `Rotate`
  (`SceneComponent.K2_AddLocalRotation` (`self.Rotator`) (`KismetMathLibrary.MakeRotator` 0.0 0.0 (`self.Rotation speed`)) false false))

(fn `UserConstructionScript`
  (if (not (`self.Enable light`))
    (`SceneComponent.SetVisibility` (`self.PointLight`) false false)))